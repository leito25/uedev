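; BP_FrontendController is a frontend player controller that sets up the menu UI when it possesses a pawn.
; On possess it creates the primary layout widget, adds it to the viewport and registers it with the C++ FrontendUISubsystem.
; An async PushSoftWidget action then pushes a tag-resolved soft widget class onto the Frontend widget stack, and the controller shows the mouse cursor.
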(event EventBeginPlay)

(event EventTick
  (params (DeltaSeconds :type Float%20%28single-precision%29)))

(event EventPossess
  (params (PossessedPawn :type Pawn%20Object%20Reference))
  (bind _returnvalue (UserInterface|CreateWidget "/Game/EPicTest/UI/Widgets/Others/WBP_CUW_PrimaryLayout.WBP_CUW_PrimaryLayout_C" self))
  (UserInterface|Viewport|AddtoViewport _returnvalue 0)
  (Class|FrontendUISubsystem|RegisterCreatedPrimaryLayoutWidget (Subsystems|GetFrontendUISubsystem) _returnvalue)
  (|PushSoftWidget self (Class|FrontendFunctionLibrary|GetFrontendSoftWidgetClassbyTag (Variables|Default|GetIn%20Widget%20Tag)) "(TagName=\"Frontend.WidgetStack.Frontend\")" true ; Async Blueprint Action
    (:then
      (Variables|Default|SetbShowMouseCursor true))))

(fn ConstructionScript)